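; BP_EggLight is a glowing egg that the player's dragon can catch and that can respawn.
; Light and catch collision volumes flag player overlap and catchability, with Tick rechecking while the player is outside the light.
; Catch hides the mesh and light, disables collision and registers the egg on BP_DragonCharacter; Respawn restores them and rechecks overlaps.
; While the player is in the light, Tick draws a debug visibility trace whose result is unused.
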(event OnComponentBeginOverlap(lightCollision)
  (params (OverlappedComponent :type Primitive%20Component%20Object%20Reference) (OtherActor :type Actor%20Object%20Reference) (OtherComp :type Primitive%20Component%20Object%20Reference) (OtherBodyIndex :type Integer) (bFromSweep :type Boolean) (SweepResult :type Hit%20Result%20Structure%20%28by%20ref%29))
  (if (== OtherActor (Game|GetPlayerCharacter 0))
    (Variables|Default|SetisPlayerOverlapped true)))

(event OnComponentEndOverlap(lightCollision)
  (params (OverlappedComponent :type Primitive%20Component%20Object%20Reference) (OtherActor :type Actor%20Object%20Reference) (OtherComp :type Primitive%20Component%20Object%20Reference) (OtherBodyIndex :type Integer))
  (if (== (Game|GetPlayerCharacter 0) OtherActor)
    (Variables|Default|SetisPlayerOverlapped false)))

(event OnComponentBeginOverlap(catchCollision)
  (params (OverlappedComponent :type Primitive%20Component%20Object%20Reference) (OtherActor :type Actor%20Object%20Reference) (OtherComp :type Primitive%20Component%20Object%20Reference) (OtherBodyIndex :type Integer) (bFromSweep :type Boolean) (SweepResult :type Hit%20Result%20Structure%20%28by%20ref%29))
  (if (== OtherActor (Game|GetPlayerCharacter 0))
    (Variables|Default|SetisCatchableByPlayer true)))

(event OnComponentEndOverlap(catchCollision)
  (params (OverlappedComponent :type Primitive%20Component%20Object%20Reference) (OtherActor :type Actor%20Object%20Reference) (OtherComp :type Primitive%20Component%20Object%20Reference) (OtherBodyIndex :type Integer))
  (if (== (Game|GetPlayerCharacter 0) OtherActor)
    (Variables|Default|SetisCatchableByPlayer false)))

(event Custom|Respawn
  (CallFunction|SetVisible)
  (CallFunction|CHeckOerlap))

(event Custom|CHeckOerlap
  (bind _array_element (Utilities|Array|ForEachLoopwithBreak (Collision|GetOverlappingActors (Variables|Default|GetlightCollision) "/Game/Characters/Dragon/BP_DragonCharacter.BP_DragonCharacter_C" :!class /Script/Engine.PrimitiveComponent) :!label _label)
    (:LoopBody
      (if (== _array_element (Game|GetPlayerCharacter 0))
        (Variables|Default|SetisPlayerOverlapped true)
        (goto _label Break)))
    (:Completed
      (bind _array_element_2 (Utilities|Array|ForEachLoopwithBreak (Collision|GetOverlappingActors (Variables|Default|GetcatchCollision) "/Game/Characters/Dragon/BP_DragonCharacter.BP_DragonCharacter_C" :!class /Script/Engine.PrimitiveComponent) :!label _label_2)
        (:LoopBody
          (if (== _array_element_2 (Game|GetPlayerCharacter 0))
            (Variables|Default|SetisCatchableByPlayer true)
            (goto _label_2 Break)))))))

(event EventTick
  (params (DeltaSeconds :type Float%20%28single-precision%29))
  ;[1 1 1] Event Tick
  (if (not (Variables|Default|GetisCatched))
    (if (Variables|Default|GetisPlayerOverlapped)
      (bind _outhit (Collision|LineTraceByChannel (Transformation|GetActorLocation) (Transformation|GetActorLocation (Game|GetPlayerCharacter 0)) "TraceTypeQuery1" false 0 "ForDuration"))
      (if (.bBlockingHit (Collision|BreakHitResult _outhit))
        _)
      (else
        (CallFunction|CHeckOerlap)))))

(event EventCatch
  (Utilities|FlowControl|DelayUntilNextTick)
  (CallFunction|SetInvisible)
  (bind _asbp_dragon_character (Utilities|Casting|CastToBP_DragonCharacter (Game|GetPlayerCharacter 0)))
  (Variables|/Game/Characters/Dragon/BP_DragonCharacter.BP_DragonCharacter_C|SeteggCatched _asbp_dragon_character self))

(fn ConstructionScript)

(fn SetVisible
  (bind _eggmesh (Variables|Default|GeteggMesh))
  (Rendering|SetVisibility _eggmesh true false)
  (Collision|SetCollisionEnabled _eggmesh "QueryAndPhysics")
  (Rendering|SetVisibility (Variables|Default|GetPointLight) true false)
  (Variables|Default|SetisCatched false))

(fn SetInvisible
  (Rendering|SetVisibility (Variables|Default|GeteggMesh) false false)
  (Rendering|SetVisibility (Variables|Default|GetPointLight) false false)
  (Collision|SetCollisionEnabled (Variables|Default|GeteggMesh) "NoCollision")
  (Variables|Default|SetisCatched true))