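; Horizontal movable platform Blueprint, by its name, though this file holds only its setup and no movement logic.
; The construction script sets the Box world scale from Size on Y with zero on X and Z, and resets StartLocation and EndLocation to the origin.
; Disconnected nodes multiply Size by the Box's relative Y for positive and negative offsets.
; SetTrigger stores a trigger reference and flags HasTrigger.
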(fn ConstructionScript
  (Transformation|SetWorldScale3D (Variables|Default|GetBox) (Math|Vector|MakeVector 0.0 (Variables|Default|Getsize) 0.0))
  (Variables|Default|SetstartLocation (Math|Vector|MakeVector 0.0 0.0 0.0))
  (Variables|Default|SetendLocation "0, 0, 0"))

(fn SetTrigger
  (params (Trigger :type BP%20Trigger%20Object%20Reference))
  (Variables|Default|SetTrigger Trigger)
  (Variables|Default|SetHasTrigger true))