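; BP_PlayerCharacter is the player character, with axis-driven movement along world Y, jumping, and picking up and dropping objects.
; The Action input attaches the first overlapping actor tagged "catchable" to the mesh's hand_socket.
; Pressing it again traces toward negative Y and downward, then detaches the held object at the hit point, keeping it held if nothing is hit.
; The "Trigger" tag check leads to no action.
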(event EventBeginPlay)

(event Collision|EventActorBeginOverlap
  (params (OtherActor :type Actor%20Object%20Reference)))

(event EventTick
  (params (DeltaSeconds :type Float%20%28single-precision%29)))

(event Input|ActionEvents|InputActionJump
  (params (Key :type Key%20Structure :default "None"))
  ;[1 1 1] Mouvements
  (:Pressed
    (Character|Jump)))

(event Input|ActionEvents|InputActionAction
  (params (Key :type Key%20Structure :default "None"))
  (:Pressed
    (if (Variables|Default|GetisCatching)
      ;[1 1 1] drop object
      (bind (_outhit _returnvalue) (Collision|LineTraceByChannel (Transformation|GetActorLocation) (- (Transformation|GetActorLocation) "0.000000,500.000000,200.000000") "TraceTypeQuery1" false 0 "None"))
      (if _returnvalue
        (Transformation|DetachFromActor (Variables|Default|GetCatchedElement) "KeepWorld" "KeepWorld" "KeepWorld")
        (Transformation|SetActorTransform (Variables|Default|GetCatchedElement) (Math|Transform|MakeTransform (.Location (Collision|BreakHitResult _outhit)) "0, 0, 0" "1.000000,1.000000,1.000000"))
        (Variables|Default|SetisCatching false))
      (else
        ;[1 1 1] Catch object
        (bind _array_element (Utilities|Array|ForEachLoopwithBreak (Collision|GetOverlappingActors 0 :!class /Script/Engine.Actor) :!label _label)
          (:LoopBody
            (if (Actor|ActorHasTag _array_element "catchable")
              (bind _output_get (Variables|Default|SetCatchedElement _array_element))
              (Transformation|AttachComponentToComponent _output_get (Variables|Character|GetMesh) "hand_socket" "KeepRelative" "KeepRelative" "KeepRelative" true)
              (Variables|Default|SetisCatching true)
              (goto _label Break)
              (elif (Actor|ActorHasTag _array_element "Trigger")
                _))))))))

(event Input|AxisEvents|InputAxisxAxis
  (params (AxisValue :type Float%20%28single-precision%29))
  ;[1 1 1] Mouvements
  (Pawn|Input|AddMovementInput "0,1.000000, 0" AxisValue false))

(fn ConstructionScript)

(fn GetPlayerCharacter
  (return self))